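; BP_Mask is a temporary portal hole actor that drives a spherical material mask through the MPC_Mask parameter collection and lets the first-person character pass through.
; On BeginPlay a timeline grows the mask radius and torus mesh, then after a long delay a second one shrinks them with the capsule and destroys the actor.
; Capsule overlaps switch the character's collision profile to "Hole", restoring "Pawn" on exit.
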(event OnComponentBeginOverlap(Capsule)
  (params (OverlappedComponent :type Primitive%20Component%20Object%20Reference) (OtherActor :type Actor%20Object%20Reference) (OtherComp :type Primitive%20Component%20Object%20Reference) (OtherBodyIndex :type Integer) (bFromSweep :type Boolean) (SweepResult :type Hit%20Result%20Structure%20%28by%20ref%29))
  (bind _asbp_first_person_character (Utilities|Casting|CastToBP_FirstPersonCharacter OtherActor))
  (Collision|SetCollisionProfileName (Variables|/Script/Engine.Character|GetCapsuleComponent _asbp_first_person_character) "Hole" false :!class /Script/Engine.PrimitiveComponent))

(event OnComponentEndOverlap(Capsule)
  (params (OverlappedComponent :type Primitive%20Component%20Object%20Reference) (OtherActor :type Actor%20Object%20Reference) (OtherComp :type Primitive%20Component%20Object%20Reference) (OtherBodyIndex :type Integer))
  (bind _asbp_first_person_character (Utilities|Casting|CastToBP_FirstPersonCharacter OtherActor))
  (Collision|SetCollisionProfileName (Variables|/Script/Engine.Character|GetCapsuleComponent _asbp_first_person_character) "Pawn" true :!class /Script/Engine.PrimitiveComponent))

(event EventBeginPlay
  (Rendering|Material|SetVectorParameterValue "/Game/FX/Portal/MPC_Mask.MPC_Mask" "Location" (Math|Conversions|ToLinearColor(Vector) (Transformation|GetWorldLocation (Variables|Default|GetSphere))) :!class /Script/Engine.KismetMaterialLibrary)
  (bind _newtrack_0 (Timeline|Timeline PlayFromStart)
    (:Update
      (Rendering|Material|SetScalarParameterValue "/Game/FX/Portal/MPC_Mask.MPC_Mask" "Radius" (Math|Float|Lerp 0.0 (Variables|Default|GetRadius) _newtrack_0) :!class /Script/Engine.KismetMaterialLibrary)
      (Transformation|SetRelativeScale3D (Variables|Default|GetShape_Torus) (Math|Vector|MakeVector (Math|Float|Lerp 0.0 1.0 _newtrack_0) (Math|Float|Lerp 0.0 1.0 _newtrack_0) 1.5)))
    (:Finished
      (Utilities|FlowControl|Delay 3e+02)
      (bind _newtrack_0_2 (Timeline|Timeline_0 PlayFromStart)
        (:Update
          (Rendering|Material|SetScalarParameterValue "/Game/FX/Portal/MPC_Mask.MPC_Mask" "Radius" (Math|Float|Lerp (Variables|Default|GetRadius) 0.0 _newtrack_0_2) :!class /Script/Engine.KismetMaterialLibrary)
          (Transformation|SetRelativeScale3D (Variables|Default|GetShape_Torus) (Math|Vector|MakeVector (Math|Float|Lerp 1.0 0.0 _newtrack_0_2) (Math|Float|Lerp 1.0 0.0 _newtrack_0_2) 1.5))
          (Transformation|SetRelativeScale3D (Variables|Default|GetCapsule) (Math|Vector|MakeVector (Math|Float|Lerp 1.0 0.0 _newtrack_0_2) (Math|Float|Lerp 1.0 0.0 _newtrack_0_2) (Math|Float|Lerp 1.0 0.0 _newtrack_0_2))))
        (:Finished
          (Actor|DestroyActor))))))

(fn ConstructionScript
  (Rendering|Material|SetVectorParameterValue "/Game/FX/Portal/MPC_Mask.MPC_Mask" "Location" (Math|Conversions|ToLinearColor(Vector) (Transformation|GetWorldLocation (Variables|Default|GetSphere))) :!class /Script/Engine.KismetMaterialLibrary)
  (Rendering|Material|SetScalarParameterValue "/Game/FX/Portal/MPC_Mask.MPC_Mask" "Radius" 1.8e+02 :!class /Script/Engine.KismetMaterialLibrary))